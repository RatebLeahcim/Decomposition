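; BP_SlabTrigger is a pressure-plate trigger that sinks and rises as tagged actors enter and leave its box.
; Overlaps are filtered against SlabTagContainer, so only the first matching actor starts the press and the slab reverses once none remain.
; The SlabDepression timeline drives the slab's relative Z.
; On finishing, it calls DepressionEndEvent if still pressed, or UndepressEvent when reversed.
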(event OnComponentBeginOverlap(Box)
  (params (OverlappedComponent :type Primitive%20Component%20Object%20Reference) (OtherActor :type Actor%20Object%20Reference) (OtherComp :type Primitive%20Component%20Object%20Reference) (OtherBodyIndex :type Integer) (bFromSweep :type Boolean) (SweepResult :type Hit%20Result%20Structure%20%28by%20ref%29))
  (if (not (CallFunction|CheckifAnyDepressors OtherActor))
    (bind _hastags (Class|BPITagHolder|HasAllMatchingTags(Message) OtherActor (Variables|Default|GetSlabTagContainer)))
    (if _hastags
      (Variables|Default|SetStillDepressing true)
      (Variables|Default|SetPlay true)
      (bind (_direction _depression_curve) (Timeline|Slab%20Depression Play)
        (:Update
          (Transformation|SetRelativeLocation (Variables|Default|GetSlab) (Math|Vector|MakeVector 0.0 0.0 _depression_curve) false false))
        (:Finished
          (Variables|Default|SetStillDepressing false)
          (switch Utilities|FlowControl|Switch|SwitchonETimelineDirection _direction
            (:Forward
              (if (Variables|Default|GetPlay)
                (Default|CallDepressionEndEvent)))
            (:Backward
              (Default|CallUndepressEvent))))))))

(event OnComponentEndOverlap(Box)
  (params (OverlappedComponent :type Primitive%20Component%20Object%20Reference) (OtherActor :type Actor%20Object%20Reference) (OtherComp :type Primitive%20Component%20Object%20Reference) (OtherBodyIndex :type Integer))
  (if (not (CallFunction|CheckifAnyDepressors))
    (Variables|Default|SetPlay false)
    (bind (_direction _depression_curve) (Timeline|Slab%20Depression Reverse)
      (:Update
        (Transformation|SetRelativeLocation (Variables|Default|GetSlab) (Math|Vector|MakeVector 0.0 0.0 _depression_curve) false false))
      (:Finished
        (Variables|Default|SetStillDepressing false)
        (switch Utilities|FlowControl|Switch|SwitchonETimelineDirection _direction
          (:Forward
            (if (Variables|Default|GetPlay)
              (Default|CallDepressionEndEvent)))
          (:Backward
            (Default|CallUndepressEvent)))))))

(fn ConstructionScript)

(fn CheckifAnyDepressors
  (params (FilterActor :type Actor%20Object%20Reference))
  (bind _array_element (Utilities|Array|ForEachLoopwithBreak (Collision|GetOverlappingActors (Variables|Default|GetBox) 0 :!class /Script/Engine.PrimitiveComponent) :!label _label)
    (:LoopBody
      (bind _hastags (Class|BPITagHolder|HasAllMatchingTags(Message) _array_element (Variables|Default|GetSlabTagContainer)))
      (if (and _hastags (!= _array_element FilterActor))
        (LocalVariables|SetFoundDepressor true)
        (goto _label Break)))
    (:Completed
      (return (LocalVariables|GetFoundDepressor)))))