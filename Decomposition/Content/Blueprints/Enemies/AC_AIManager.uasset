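; AC_AIManager is an enemy AI component that supplies patrol points.
; On BeginPlay it caches every BP_PatrolPoint actor in the level.
; GetPatrolPoints filters that cached list by the requested patrol group enum.
; GetSpecificPoint returns a random point from whichever point list it receives.
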(event EventBeginPlay
  (bind _outactors (Actor|GetAllActorsOfClass "/Game/Blueprints/Enemies/BP_PatrolPoint.BP_PatrolPoint_C"))
  (Variables|Default|SetAllPatrolPoints _outactors))

(event EventTick
  (params (DeltaSeconds :type Float%20%28single-precision%29)))

(fn GetPatrolPoints
  (params (PatrolGroup :type E_PatrolGroups%20Enum :default "NewEnumerator1"))
  (bind _groupedpoints (LocalVariables|GetGroupedPoints))
  (for _array_element (Variables|Default|GetAllPatrolPoints)
    (if (Utilities|Enum|Equal(Enum) PatrolGroup (Variables|/Game/Blueprints/Enemies/BP_PatrolPoint.BP_PatrolPoint_C|GetE_PatrolGroup _array_element))
      (Utilities|Array|Add _groupedpoints _array_element)))
  (return _groupedpoints))

(fn GetSpecificPoint
  (params (PatrolPoints :type Array%20of%20BP%20Patrol%20Point%20Object%20References))
  (return (.OutItem (Utilities|Array|Random PatrolPoints))))