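; Prototype actor for an immersive portal view, pairing a camera that follows the player with an alternate one at a second portal.
; BeginPlay caches the locations of the first two BP_Portal actors found in the level.
; Each Tick copies the player camera transform to PlayerCam, then places AlterCam at Portal2 plus the Portal1-minus-camera offset, sharing the player's rotation.
; Debug boxes mark both cameras every frame.
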(event EventTick
  (params (DeltaSeconds :type Float%20%28single-precision%29))
  (bind _playercam (Variables|Default|GetPlayerCam))
  (bind _portal1pos (Variables|Default|GetPortal1Pos))
  (bind _portal2pos (Variables|Default|GetPortal2Pos))
  (bind _returnvalue (Transformation|GetWorldLocation _playercam))
  (Transformation|SetWorldTransform _playercam (Transformation|GetActorTransform (Game|GetPlayerCameraManager 0)) false false)
  (Rendering|Debug|DrawDebugBox :Center (Transformation|GetWorldLocation (Variables|Default|GetPlayerCam)) :Extent "10.000000,10.000000,10.000000" :Thickness 1e+01)
  (Transformation|SetWorldTransform (Variables|Default|GetAlterCam) (Math|Transform|MakeTransform (Math|Vector|MakeVector (+ (- (.x _portal1pos) (.x _returnvalue)) (.x _portal2pos)) (+ (- (.y _portal1pos) (.y _returnvalue)) (.y _portal2pos)) (+ (- (.z _portal1pos) (.z _returnvalue)) (.z _portal2pos))) (Camera|GetCameraRotation (Game|GetPlayerCameraManager 0)) "1.000000,1.000000,1.000000") false false)
  (Rendering|Debug|DrawDebugBox :Center (Transformation|GetWorldLocation (Variables|Default|GetAlterCam)) :Extent "10.000000,10.000000,10.000000" :Thickness 1e+01))

(event EventBeginPlay
  (bind _outactors (Actor|GetAllActorsOfClass "/Game/Blueprints/RandomEvent/HelpersBP/BP_Portal.BP_Portal_C"))
  (Utilities|FlowControl|Sequence
    (:then_0
      (Variables|Default|SetPortal1Pos (Transformation|GetActorLocation (Utilities|Array|Get(acopy) _outactors))))
    (:then_1
      (Variables|Default|SetPortal2Pos (Transformation|GetActorLocation (Utilities|Array|Get(acopy) _outactors 1))))))

(fn ConstructionScript)