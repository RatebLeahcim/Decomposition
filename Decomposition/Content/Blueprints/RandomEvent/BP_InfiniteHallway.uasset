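; Random event that creates an infinite hallway by looping the player between two portals.
; SetupEvent spawns Red and Blue portals at PortalDistance either side of the player along world X, and TriggerEvent binds both overlaps to one handler.
; Only Red overlaps teleport the player, moving them to Blue's X while keeping Y and Z.
; Each tick, a SceneCaptureComponent2D copies the player camera's location and rotation.
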(event Custom|OnActorBeginOverlap_Event
  (params (OverlappedActor :type Actor%20Object%20Reference) (OtherActor :type Actor%20Object%20Reference))
  (bind _returnvalue (Game|Player|GetPlayerPawn 0))
  (bind _returnvalue_2 (Transformation|GetActorLocation _returnvalue))
  (if (== OverlappedActor (Variables|Default|GetRedPortal))
    (Transformation|SetActorLocation _returnvalue (Math|Vector|MakeVector (.x (Transformation|GetActorLocation (Variables|Default|GetBluePortal))) (.y _returnvalue_2) (.z _returnvalue_2)) false false)))

(event EventTriggerEvent
  (EventDispatchers|AssignOnActorBeginOverlap (Variables|Default|GetRedPortal) (delegate Custom|OnActorBeginOverlap_Event))
  (Collision|BindEventtoOnActorBeginOverlap (Variables|Default|GetBluePortal) (delegate Custom|OnActorBeginOverlap_Event)))

(event EventTick
  (params (DeltaSeconds :type Float%20%28single-precision%29))
  (bind _returnvalue (Game|GetPlayerCameraManager 0))
  (bind _scenecapturecomponent2d (Variables|Default|GetSceneCaptureComponent2D))
  (bind _returnvalue_2 (Transformation|GetActorLocation _returnvalue))
  ;[1 1 1] CaptureComponent set on Player
  (Transformation|SetWorldLocation _scenecapturecomponent2d (Math|Vector|MakeVector (.x _returnvalue_2) (.y _returnvalue_2) (.z _returnvalue_2)) false false)
  (Transformation|SetWorldRotation _scenecapturecomponent2d (Transformation|GetActorRotation _returnvalue) false false))

(event EventSetupEvent
  (bind _returnvalue (Game|Player|GetPlayerPawn 0))
  (bind _returnvalue_2 (Game|Player|GetPlayerPawn 0))
  (bind _returnvalue_3 (Transformation|GetActorLocation _returnvalue))
  (bind _returnvalue_4 (Transformation|GetActorLocation _returnvalue_2))
  ;[1 1 1] Create Red and Blue Portals
  (bind _returnvalue_5 (Game|SpawnActorfromClass "/Game/Blueprints/RandomEvent/HelpersBP/BP_Portal.BP_Portal_C" (Math|Transform|MakeTransform (Math|Vector|MakeVector (+ (Variables|Default|GetPortalDistance) (.x _returnvalue_4)) (.y _returnvalue_4) (.z _returnvalue_4)) "0, 0, 0" "1.000000,1.000000,1.000000") "Undefined" "MultiplyWithRoot" 0 0))
  (Variables|Default|SetRedPortal _returnvalue_5)
  (bind _returnvalue_6 (Game|SpawnActorfromClass "/Game/Blueprints/RandomEvent/HelpersBP/BP_Portal.BP_Portal_C" (Math|Transform|MakeTransform (Math|Vector|MakeVector (- (.x _returnvalue_3) (Variables|Default|GetPortalDistance)) (.y _returnvalue_3) (.z _returnvalue_3)) "0, 0, 0" "1.000000,1.000000,1.000000") "Undefined" "MultiplyWithRoot" 0 0))
  (Variables|Default|SetBluePortal _returnvalue_6))

(fn ConstructionScript)