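; Random event actor that surrounds the player with a slowly rotating swarm of eyeballs for a limited time.
; Sequence spawns EyeballCount BP_Eye actors at random offsets scaled by SpawnRadius and attaches them to this actor with relative transforms.
; Tick moves the actor to the player pawn and increments its yaw, carrying the eyes along.
; After EventDuration, EndEvent destroys all BP_Eye actors and itself.
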(event EventBeginPlay)

(event Collision|EventActorBeginOverlap
  (params (OtherActor :type Actor%20Object%20Reference)))

(event EventTick
  (params (DeltaSeconds :type Float%20%28single-precision%29))
  (Transformation|SetActorLocation (Transformation|GetActorLocation (Game|Player|GetPlayerPawn 0)) false false)
  (Transformation|SetActorRotation (Math|Rotator|MakeRotator 0.0 0.0 (+ (.yaw (Transformation|GetWorldRotation (Variables|Default|GetDefaultSceneRoot))) 0.5))))

(event EventSequence
  (CallFunction|SetupEvent)
  (CallFunction|TriggerEvent)
  (Utilities|FlowControl|Delay (Variables|Default|GetEventDuration))
  (CallFunction|EndEvent))

(event EventSetupEvent)

(event EventTriggerEvent
  (bind _returnvalue (Math|Trig|GetPI))
  (bind _returnvalue_2 (* _returnvalue 2.0))
  (bind _returnvalue_3 (Math|Random|RandomFloatinRange 0.0 _returnvalue_2))
  (for _index (range 0 (- (Variables|Default|GetEyeballCount) 1))
    (bind _returnvalue_4 (Game|SpawnActorfromClass "/Game/Blueprints/RandomEvent/HelpersBP/BP_Eye.BP_Eye_C" (Math|Conversions|ToTransform(Vector) (+ (Math|Vector|MakeVector 0.0 0.0 0.0) (Math|Vector|MakeVector (* (Variables|Default|GetSpawnRadius) (Math|Trig|Cos(Radians) _returnvalue_3)) (* (Variables|Default|GetSpawnRadius) (Math|Trig|Sin(Radians) _returnvalue_3)) (Math|Random|RandomFloatinRange 5.0 2e+02)))) "Undefined" "MultiplyWithRoot" 0 0))
    (bind _returnvalue_5 (Actor|GetActorOfClass "BP_Eyeballs_C"))
    (Transformation|AttachActorToActor _returnvalue_4 _returnvalue_5 "None" "KeepRelative" "KeepRelative" "KeepRelative" true)))

(event EventEndEvent
  (bind _outactors (Actor|GetAllActorsOfClass "/Game/Blueprints/RandomEvent/HelpersBP/BP_Eye.BP_Eye_C"))
  (for _array_element _outactors
    (Actor|DestroyActor _array_element)
    (Actor|DestroyActor)))

(fn ConstructionScript)