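; Generic, reusable interaction component that lets any interactable respond to a tool's hover, interact, use, pick-up, drop and cancel actions.
; Most actions are filtered by the tool's mode against allowed interaction or use lists, then relayed through event calls for owner-specific logic without subclassing.
; Hover shows the tool's interaction message and toggles outlines through custom depth stencil values.
; The enable flag gates only hover and interaction begin/end.
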(event EventBeginPlay)

(event EventTick
  (params (DeltaSeconds :type Float%20%28single-precision%29)))

(event EventCancelInteraction
  (params (Tool :type AC%20Tool%20Component%20Object%20Reference))
  ;[0.05098 0.05098 0.05098] These events are so that the same generic InteractionComponent can be reused on any interactable, allowing them to implement custom logic without creating a new InteractionComponent subclass. You can still do this if you require more custom behavior however.
  (Variables|Default|SetbIsInteracting false)
  (Default|CallInteractionCancelEvent Tool))

(event EventUse
  (params (Tool :type AC%20Tool%20Component%20Object%20Reference))
  ;[0.05098 0.05098 0.05098] These events are so that the same generic InteractionComponent can be reused on any interactable, allowing them to implement custom logic without creating a new InteractionComponent subclass. You can still do this if you require more custom behavior however.
  (if (Utilities|Array|ContainsItem (Variables|Default|GetAllowedUseTools) (Variables|/Game/Blueprints/Interaction/AC_ToolComponent.AC_ToolComponent_C|GetToolMode Tool))
    (Default|CallUseItemEvent Tool)))

(event EventMouseOver
  (params (Tool :type AC%20Tool%20Component%20Object%20Reference))
  ;[0.05098 0.05098 0.05098] These events are so that the same generic InteractionComponent can be reused on any interactable, allowing them to implement custom logic without creating a new InteractionComponent subclass. You can still do this if you require more custom behavior however.
  (if (and (Utilities|Array|ContainsItem (Variables|Default|GetAllowedInteractionTools) (Variables|/Game/Blueprints/Interaction/AC_ToolComponent.AC_ToolComponent_C|GetToolMode Tool)) (Variables|Default|GetbInteractionEnabled))
    (CallFunction|ShowOutlines)
    (Default|SetInteractionUI Tool (Variables|ItemSettings|GetInteractionMessage))))

(event EventMouseExit
  (params (Tool :type AC%20Tool%20Component%20Object%20Reference))
  ;[0.05098 0.05098 0.05098] These events are so that the same generic InteractionComponent can be reused on any interactable, allowing them to implement custom logic without creating a new InteractionComponent subclass. You can still do this if you require more custom behavior however.
  (CallFunction|HideOutlines)
  (Default|HideInteractionUI Tool))

(event EventInteractionBegin
  (params (Tool :type AC%20Tool%20Component%20Object%20Reference))
  ;[0.05098 0.05098 0.05098] These events are so that the same generic InteractionComponent can be reused on any interactable, allowing them to implement custom logic without creating a new InteractionComponent subclass. You can still do this if you require more custom behavior however.
  (if (and (Utilities|Array|ContainsItem (Variables|Default|GetAllowedInteractionTools) (Variables|/Game/Blueprints/Interaction/AC_ToolComponent.AC_ToolComponent_C|GetToolMode Tool)) (Variables|Default|GetbInteractionEnabled))
    (Default|CallInteractionBeginEvent Tool)
    (Variables|Default|SetbIsInteracting true)))

(event EventInteractionEnd
  (params (Tool :type AC%20Tool%20Component%20Object%20Reference))
  ;[0.05098 0.05098 0.05098] These events are so that the same generic InteractionComponent can be reused on any interactable, allowing them to implement custom logic without creating a new InteractionComponent subclass. You can still do this if you require more custom behavior however.
  (if (and (Utilities|Array|ContainsItem (Variables|Default|GetAllowedInteractionTools) (Variables|/Game/Blueprints/Interaction/AC_ToolComponent.AC_ToolComponent_C|GetToolMode Tool)) (Variables|Default|GetbInteractionEnabled))
    (Default|CallInteractionEndEvent Tool)
    (Variables|Default|SetbIsInteracting false)))

(event EventPickUp
  (params (Tool :type AC%20Tool%20Component%20Object%20Reference))
  ;[0.05098 0.05098 0.05098] These events are so that the same generic InteractionComponent can be reused on any interactable, allowing them to implement custom logic without creating a new InteractionComponent subclass. You can still do this if you require more custom behavior however.
  (if (Utilities|Array|ContainsItem (Variables|Default|GetAllowedInteractionTools) (Variables|/Game/Blueprints/Interaction/AC_ToolComponent.AC_ToolComponent_C|GetToolMode Tool))
    (Default|CallPickUpEvent Tool)
    (Variables|Default|SetbHeld true)))

(event EventDrop
  (params (Tool :type AC%20Tool%20Component%20Object%20Reference))
  ;[0.05098 0.05098 0.05098] These events are so that the same generic InteractionComponent can be reused on any interactable, allowing them to implement custom logic without creating a new InteractionComponent subclass. You can still do this if you require more custom behavior however.
  (if (Utilities|Array|ContainsItem (Variables|Default|GetAllowedUseTools) (Variables|/Game/Blueprints/Interaction/AC_ToolComponent.AC_ToolComponent_C|GetToolMode Tool))
    (Default|CallDropEvent Tool)
    (Variables|Default|SetbHeld false)))

(fn ShowInteractionUI)

(fn ShowOutlines
  (if (not (Variables|Default|GetbOutlineEnabled))
    (for _array_element (Variables|Default|GetOutlineObjects)
      (Rendering|SetRenderCustomDepth _array_element true)
      (Rendering|SetCustomDepthStencilValue _array_element 1))
    (Variables|Default|SetbOutlineEnabled true)))

(fn HideOutlines
  (if (Variables|Default|GetbOutlineEnabled)
    (for _array_element (Variables|Default|GetOutlineObjects)
      (Rendering|SetRenderCustomDepth _array_element true)
      (Rendering|SetCustomDepthStencilValue _array_element 0))
    (Variables|Default|SetbOutlineEnabled false)))

(fn EnableInteraction
  (Variables|Default|SetbInteractionEnabled true))

(fn DisableInteraction
  (Variables|Default|SetbInteractionEnabled false))