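; Player interaction component that targets, triggers and holds objects implementing I_Interactable, and drives an interaction prompt widget.
; Each Tick, unless ToolMode blocks it, a camera line trace sends mouse over/exit and cancel messages to the first interactable component on the hit actor.
; Interact, Use and Drop inputs message the current or held interactable.
; It holds one item at a time and shows current and held names as debug UI.
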(event Input|EnhancedActionEvents|EnhancedInputActionIA_Interact
  (params (ActionValue :type Boolean) (ElapsedSeconds :type Float%20%28double-precision%29) (TriggeredSeconds :type Float%20%28double-precision%29) (InputAction :type Input%20Action%20Object%20Reference :default "/Game/Input/Actions/IA_Interact.IA_Interact"))
  (bind _self self)
  ;[0.05098 0.05098 0.05098] Trigger interactions
  (:Started
    (Utilities|IsValid (Utilities|ToObject(Interface) (Variables|Default|GetCurrentInteractable))
      (:Is%20Valid
        (Class|IInteractable|InteractionBegin(Message) (Utilities|ToObject(Interface) (Variables|Default|GetCurrentInteractable)) _self))))
  (:Completed
    (Utilities|IsValid (Utilities|ToObject(Interface) (Variables|Default|GetCurrentInteractable))
      (:Is%20Valid
        (Class|IInteractable|InteractionEnd(Message) (Utilities|ToObject(Interface) (Variables|Default|GetCurrentInteractable)) _self)
        (Variables|Default|SetCurrentInteractable 0)))))

(event Input|EnhancedActionEvents|EnhancedInputActionIA_Use
  (params (ActionValue :type Boolean) (ElapsedSeconds :type Float%20%28double-precision%29) (TriggeredSeconds :type Float%20%28double-precision%29) (InputAction :type Input%20Action%20Object%20Reference :default "/Game/Input/Actions/IA_Use.IA_Use"))
  (bind _heldinteractable (Variables|Default|GetHeldInteractable))
  (bind _returnvalue (Utilities|ToObject(Interface) _heldinteractable))
  ;[0.05098 0.05098 0.05098] Trigger interactions
  (:Completed
    (Utilities|IsValid _returnvalue
      (:Is%20Valid
        (Class|IInteractable|Use(Message) _returnvalue self)))))

(event Input|EnhancedActionEvents|EnhancedInputActionIA_Drop
  (params (ActionValue :type Boolean) (ElapsedSeconds :type Float%20%28double-precision%29) (TriggeredSeconds :type Float%20%28double-precision%29) (InputAction :type Input%20Action%20Object%20Reference :default "/Game/Input/Actions/IA_Drop.IA_Drop"))
  (bind _heldinteractable (Variables|Default|GetHeldInteractable))
  (bind _returnvalue (Utilities|ToObject(Interface) _heldinteractable))
  ;[0.05098 0.05098 0.05098] Trigger interactions
  (:Completed
    (Utilities|IsValid _returnvalue
      (:Is%20Valid
        (Class|IInteractable|Drop(Message) _returnvalue self)))))

(event EventBeginPlay
  (bind _returnvalue (UserInterface|CreateWidget "/Game/Blueprints/Interaction/WBP_InteractionUI.WBP_InteractionUI_C"))
  (bind _output_get (Variables|Default|SetInteractionUI _returnvalue))
  (UserInterface|Viewport|AddtoViewport _output_get 0))

(event EventTick
  (params (DeltaSeconds :type Float%20%28single-precision%29))
  (bind _returnvalue (Game|GetPlayerCameraManager 0))
  (bind _self self)
  (bind _returnvalue_2 (Camera|GetCameraLocation _returnvalue))
  ;[0.05098 0.05098 0.05098] Trace for interactables and trigger mouse over/exit events
  (CallFunction|UpdateDebugUI)
  (if (Utilities|Enum|NotEqual(Enum) (Variables|Default|GetToolMode) "NewEnumerator1")
    (bind (_outhit _returnvalue_3) (Collision|LineTraceByChannel _returnvalue_2 (+ _returnvalue_2 (* (Transformation|GetActorForwardVector _returnvalue) (Variables|Default|GetInteractionDistance))) "TraceTypeQuery3" false 0 "None"))
    (if _returnvalue_3
      (Utilities|IsValid (Utilities|ToObject(Interface) (Variables|Default|GetCurrentInteractable))
        (:Is%20Valid
          (Class|IInteractable|MouseExit(Message) (Utilities|ToObject(Interface) (Variables|Default|GetCurrentInteractable)) self))
        (:Is%20Not%20Valid
          _))
      (if (Utilities|Array|IsNotEmpty (Class|Actor|GetComponentsbyInterface (.HitActor (Collision|BreakHitResult _outhit)) "/Game/Blueprints/Interaction/I_Interactable.I_Interactable_C"))
        ;;[0.05098 0.05098 0.05098] IsValid check is required since an object may not have any interactables
        (bind _output_get (Variables|Default|SetCurrentInteractable (.AsI%20Interactable (Utilities|Casting|CastToI_Interactable (Utilities|Array|Get(acopy) (Class|Actor|GetComponentsbyInterface (.HitActor (Collision|BreakHitResult _outhit)) "/Game/Blueprints/Interaction/I_Interactable.I_Interactable_C"))))))
        (Utilities|IsValid (Utilities|ToObject(Interface) _output_get)
          (:Is%20Valid
            (Class|IInteractable|MouseOver(Message) (Utilities|ToObject(Interface) _output_get) self))))
      (else
        (CallFunction|HideInteractionUI)
        (Utilities|IsValid (Utilities|ToObject(Interface) (Variables|Default|GetCurrentInteractable))
          (:Is%20Valid
            (if (!= (Utilities|ToObject(Interface) (Variables|Default|GetCurrentInteractable)) (Utilities|ToObject(Interface) (Variables|Default|GetHeldInteractable)))
              (Class|IInteractable|CancelInteraction(Message) (Utilities|ToObject(Interface) (Variables|Default|GetCurrentInteractable)) _self))
            (Class|IInteractable|MouseExit(Message) (Utilities|ToObject(Interface) (Variables|Default|GetCurrentInteractable)) _self)
            (Variables|Default|SetCurrentInteractable 0)))))))

(fn SetInteractionUI
  (params (Text :type String))
  (Default|SetInteractionText (Variables|Default|GetInteractionUI) Text))

(fn HideInteractionUI
  (Default|HideInteractionUI (Variables|Default|GetInteractionUI)))

(fn SetToolMode
  (params (New%20Mode :type E_ToolMode%20Enum :default "NewEnumerator0"))
  (Variables|Default|SetToolMode New%20Mode))

(fn HoldInteractable
  (params (Interactable :type I%20Interactable%20Interface))
  (CallFunction|DropInteractable)
  (bind _output_get (Variables|Default|SetHeldInteractable Interactable))
  (Default|PickUp _output_get self))

(fn DropInteractable
  (Utilities|IsValid (Utilities|ToObject(Interface) (Variables|Default|GetHeldInteractable))
    (:Is%20Valid
      (Default|Drop (Variables|Default|GetHeldInteractable) self))
    (:Is%20Not%20Valid
      _))
  (Variables|Default|SetHeldInteractable 0) ; Clear Held Interactable
)

(fn UpdateDebugUI
  (bind _interactionui (Variables|Default|GetInteractionUI))
  (bind _interactionui_2 (Variables|Default|GetInteractionUI))
  (bind _currentinteractable (Variables|Default|GetCurrentInteractable))
  (bind _heldinteractable (Variables|Default|GetHeldInteractable))
  (bind _returnvalue (Utilities|ToObject(Interface) _heldinteractable))
  (bind _returnvalue_2 (Utilities|ToObject(Interface) _currentinteractable))
  (Utilities|FlowControl|Sequence
    (:then_0
      (Utilities|IsValid _returnvalue_2
        (:Is%20Valid
          (Default|SetCurrent _interactionui_2 (Utilities|Text|ToText(String) (Utilities|GetDisplayName _returnvalue_2))))
        (:Is%20Not%20Valid
          (Default|SetCurrent _interactionui_2 "None"))))
    (:then_1
      (Utilities|IsValid _returnvalue
        (:Is%20Valid
          (Default|SetHeld _interactionui (Utilities|Text|ToText(String) (Utilities|GetDisplayName _returnvalue))))
        (:Is%20Not%20Valid
          (Default|SetHeld _interactionui "None"))))))