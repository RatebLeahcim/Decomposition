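; BP_FuelCell is an interactable pickup that supplies a fuel cell to the lantern.
; On BeginPlay it registers its cube as the interaction component's outline object and tints it orange through a dynamic material instance.
; When an interaction ends, it calls AddFuelCell on the first BP_Lantern found in the world and destroys itself, staying in place if none exists.
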(event InteractionEndEvent(AC_InteractionComponent)
  (params (Tool :type AC%20Tool%20Component%20Object%20Reference))
  (bind _outactors (Actor|GetAllActorsOfClass "/Game/Blueprints/Interaction/Interactables/BP_Lantern.BP_Lantern_C"))
  (if (Utilities|Array|IsNotEmpty _outactors)
    (Default|AddFuelCell (Utilities|Array|Get(acopy) _outactors))
    (Actor|DestroyActor)))

(event EventBeginPlay
  (CallFunction|Setup))

(event Collision|EventActorBeginOverlap
  (params (OtherActor :type Actor%20Object%20Reference)))

(event EventTick
  (params (DeltaSeconds :type Float%20%28single-precision%29)))

(fn ConstructionScript)

(fn Setup
  (bind _cube (Variables|Default|GetCube))
  (Variables|/Game/Blueprints/Interaction/AC_InteractionComponent.AC_InteractionComponent_C|SetOutlineObjects (Variables|Default|GetAC_InteractionComponent) (Utilities|Array|MakeArray (Variables|Default|GetCube)))
  (bind _returnvalue (Rendering|Material|CreateDynamicMaterialInstance _cube 0 (Rendering|Material|GetMaterial _cube 0) "None" :!class /Script/Engine.PrimitiveComponent))
  (Rendering|Material|SetVectorParameterValue _returnvalue "Color" "(R=1.000000,G=0.564706,B=0.000000,A=1.000000)" :!class /Script/Engine.MaterialInstanceDynamic))