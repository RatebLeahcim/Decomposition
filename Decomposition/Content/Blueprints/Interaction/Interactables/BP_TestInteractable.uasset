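; BP_TestInteractable is a test interactable actor that exercises the interaction component on a Cube mesh.
; On BeginPlay it registers the Cube as the component's outline object, and Tick prints a debug message while an interaction is active.
; When the interaction ends, it creates a dynamic material instance from the Cube's current material and sets its Color parameter to a random color.
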(event InteractionEndEvent(AC_InteractionComponent)
  (params (Tool :type AC%20Tool%20Component%20Object%20Reference))
  (bind _cube (Variables|Default|GetCube))
  (bind _returnvalue (Rendering|Material|CreateDynamicMaterialInstance _cube 0 (Rendering|Material|GetMaterial _cube 0) "None" :!class /Script/Engine.PrimitiveComponent))
  (Rendering|Material|SetVectorParameterValue _returnvalue "Color" (Math|Color|MakeColor (Math|Random|RandomFloat) (Math|Random|RandomFloat) (Math|Random|RandomFloat)) :!class /Script/Engine.MaterialInstanceDynamic))

(event EventBeginPlay
  (Variables|/Game/Blueprints/Interaction/AC_InteractionComponent.AC_InteractionComponent_C|SetOutlineObjects (Variables|Default|GetAC_InteractionComponent) (Utilities|Array|MakeArray (Variables|Default|GetCube))))

(event Collision|EventActorBeginOverlap
  (params (OtherActor :type Actor%20Object%20Reference)))

(event EventTick
  (params (DeltaSeconds :type Float%20%28single-precision%29))
  (if (Variables|/Game/Blueprints/Interaction/AC_InteractionComponent.AC_InteractionComponent_C|GetbIsInteracting (Variables|Default|GetAC_InteractionComponent))
    (Development|PrintString "Interacting!" true true "(R=0.000000,G=0.660000,B=1.000000,A=1.000000)" 0.1)))

(fn ConstructionScript)