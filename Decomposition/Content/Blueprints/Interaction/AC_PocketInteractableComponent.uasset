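; Interactable component for items that can be picked up and stored in the player's pockets.
; Pocket add, remove, put and pull events track the InPocket state and forward to matching event calls, with removal of a held item making the pocket component's tool drop it.
; Pickup sets Held, which suppresses repeat pickups and the parent's hover and interaction handling.
; The pockets component is lazily fetched from BP_PlayerCharacter and cached.
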(event EventBeginPlay)

(event EventTick
  (params (DeltaSeconds :type Float%20%28single-precision%29)))

(event EventPickUp
  (params (Tool :type AC%20Tool%20Component%20Object%20Reference))
  (if (not (Variables|Default|GetbHeld))
    (Default|CallPickUpEvent Tool)
    (Variables|Default|SetbHeld true)))

(event EventOnAddtoPocket
  (params (Pocket :type AC%20Pockets%20Component%20Object%20Reference))
  (Default|CallAddtoPocketEvent Pocket)
  (Variables|Default|SetbInPocket true))

(event EventPutinPocket
  (params (Pocket :type AC%20Pockets%20Component%20Object%20Reference))
  (Default|CallPutinPocketEvent Pocket)
  (Variables|Default|SetbInPocket true))

(event EventPullfromPocket
  (params (Pocket :type AC%20Pockets%20Component%20Object%20Reference))
  (Default|CallPullfromPocketEvent Pocket)
  (Variables|Default|SetbInPocket false))

(event EventOnRemovefromPocket
  (params (Pocket :type AC%20Pockets%20Component%20Object%20Reference))
  (bind _pockets (CallFunction|GetPocketComponent))
  (bind _tool (Variables|/Game/Blueprints/Interaction/AC_PocketsComponent.AC_PocketsComponent_C|GetTool _pockets))
  (Variables|Default|SetbInPocket false)
  (if (Variables|Default|GetbHeld)
    (Utilities|IsValid _tool
      (:Is%20Valid
        (Default|DropInteractable _tool))
      (:Is%20Not%20Valid
        _)))
  (Default|CallRemovefromPocketEvent Pocket))

(event EventMouseOver
  (params (Tool :type AC%20Tool%20Component%20Object%20Reference))
  (if (not (Variables|Default|GetbHeld))
    (|CallParentFunction Tool)))

(event EventMouseExit
  (params (Tool :type AC%20Tool%20Component%20Object%20Reference))
  (if (not (Variables|Default|GetbHeld))
    (|CallParentFunction Tool)))

(event EventInteractionBegin
  (params (Tool :type AC%20Tool%20Component%20Object%20Reference))
  (if (not (Variables|Default|GetbHeld))
    (|CallParentFunction Tool)))

(event EventInteractionEnd
  (params (Tool :type AC%20Tool%20Component%20Object%20Reference))
  (if (not (Variables|Default|GetbHeld))
    (|CallParentFunction Tool)))

(fn GetPocketComponent
  (Utilities|IsValid (Variables|Default|GetPockets)
    (:Is%20Valid
      (return (Variables|Default|GetPockets)))
    (:Is%20Not%20Valid
      (bind _asbp_player_character (Utilities|Casting|CastToBP_PlayerCharacter (Game|GetPlayerCharacter 0))
        (:then
          (bind _output_get (Variables|Default|SetPockets (Variables|/Game/Blueprints/Player/BP_PlayerCharacter.BP_PlayerCharacter_C|GetAC_PocketsComponent _asbp_player_character)))
          (return _output_get))
        (:CastFailed
          (return 0))))))