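; Pockets component that stores a limited set of items and tracks which are currently pulled out.
; Pulling requires open pockets and, at the out-of-pocket limit, first puts the earliest pulled item back.
; Items receive add, remove, pull and put-away calls, with index-based variants for most operations.
; Closing pockets loops pulled items back in while shrinking that same array; Tick refreshes an optional debug text UI.
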(event EventBeginPlay)

(event EventTick
  (params (DeltaSeconds :type Float%20%28single-precision%29))
  (CallFunction|UpdateDebugUI))

(fn AddPocketItem
  (params (Item :type I%20Pocket%20Item%20Interface))
  (if (< (Utilities|Array|Length (Variables|Default|GetPocketItems)) (Variables|Default|GetPocketLimit))
    (Utilities|Array|Add (Variables|Default|GetPocketItems) Item)
    (Default|OnAddtoPocket Item self)
    (return true)
    (else
      (return false))))

(fn RemovePocketItem
  (params (Item :type I%20Pocket%20Item%20Interface))
  (if (Utilities|Array|ContainsItem (Variables|Default|GetPocketItems) Item)
    (Utilities|Array|RemoveItem (Variables|Default|GetOutOfPocketItems) Item)
    (bind _returnvalue (Utilities|Array|RemoveItem (Variables|Default|GetPocketItems) Item))
    (if _returnvalue
      (Default|OnRemovefromPocket Item self)
      (return true)
      (else
        (return false)))
    (else
      (return false))))

(fn RemovePocketItemIndex
  (params (Item :type Integer))
  (if (Utilities|Array|IsValidIndex (Variables|Default|GetPocketItems) Item)
    (bind _success (CallFunction|RemovePocketItem (Utilities|Array|Get(acopy) (Variables|Default|GetPocketItems) Item)))
    (return _success)
    (else
      (return false))))

(fn PullPocketItem
  (params (Item :type I%20Pocket%20Item%20Interface))
  (if (and (Utilities|Array|ContainsItem (Variables|Default|GetPocketItems) Item) (Variables|Default|GetbPocketsOpen))
    (if (< (Utilities|Array|Length (Variables|Default|GetOutOfPocketItems)) (Variables|Default|GetOutOfPocketLimit))
      _
      (elif (Utilities|Array|IsValidIndex (Variables|Default|GetOutOfPocketItems))
        (CallFunction|PutIteminPocket (Utilities|Array|Get(acopy) (Variables|Default|GetOutOfPocketItems)))
        (else
          (return false))))
    (Default|PullfromPocket Item self)
    (Utilities|Array|Add (Variables|Default|GetOutOfPocketItems) Item)
    (return true)
    (else
      (return false))))

(fn PullPocketItemIndex
  (params (Item :type Integer))
  (if (Utilities|Array|IsValidIndex (Variables|Default|GetPocketItems) Item)
    (bind _success (CallFunction|PullPocketItem (Utilities|Array|Get(acopy) (Variables|Default|GetPocketItems) Item)))
    (return _success)
    (else
      (return false))))

(fn PutIteminPocket
  (params (Item :type I%20Pocket%20Item%20Interface))
  (if (Utilities|Array|ContainsItem (Variables|Default|GetPocketItems) Item)
    (Default|PutinPocket Item self)
    (Utilities|Array|RemoveItem (Variables|Default|GetOutOfPocketItems) Item)
    (return true)
    (else
      (return false))))

(fn PutItemIndexinPocket
  (params (Index :type Integer))
  (if (Utilities|Array|IsValidIndex (Variables|Default|GetPocketItems) Index)
    (bind _success (CallFunction|PutIteminPocket (Utilities|Array|Get(acopy) (Variables|Default|GetPocketItems) Index)))
    (return _success)
    (else
      (return false))))

(fn Setup
  (params (ToolComponent :type AC%20Tool%20Component%20Object%20Reference))
  (Variables|Default|SetTool ToolComponent))

(fn DoPocketsContainItem
  (params (Item :type I%20Pocket%20Item%20Interface))
  (return (Utilities|Array|ContainsItem (Variables|Default|GetPocketItems) Item)))

(fn UpdateDebugUI
  (Utilities|IsValid (Variables|Default|GetDebugUI)
    (:Is%20Valid
      (Utilities|FlowControl|Sequence
        (:then_0
          (LocalVariables|SetOutText (Utilities|String|Append "Pocket Limit: " (Utilities|String|ToString(Integer) (Variables|Default|GetPocketLimit)) " 
" "OutOfPocket Limit: " (Utilities|String|ToString(Integer) (Variables|Default|GetOutOfPocketLimit)) " 
" "Current Pocket Items: " " 
")))
        (:then_1
          ;[0.05098 0.05098 0.05098] Pocket Items Text
          (for _array_element (Variables|Default|GetPocketItems)
            (LocalVariables|SetOutText (Utilities|String|Append (LocalVariables|GetOutText) (Utilities|GetDisplayName (Utilities|ToObject(Interface) _array_element)) " 
")))
          (LocalVariables|SetOutText (Utilities|String|Append (LocalVariables|GetOutText) " 
" "Out of Pocket Items: " " 
")))
        (:then_2
          ;[0.05098 0.05098 0.05098] Out of Pocket Items Text
          (for _array_element_2 (Variables|Default|GetOutOfPocketItems)
            (LocalVariables|SetOutText (Utilities|String|Append (LocalVariables|GetOutText) (Utilities|GetDisplayName (Utilities|ToObject(Interface) _array_element_2)) " 
"))))
        (:then_3
          (Default|UpdatePocketText (Variables|Default|GetDebugUI) (Utilities|Text|ToText(String) (LocalVariables|GetOutText))))))))

(fn OpenPockets
  (Variables|Default|SetbPocketsOpen true))

(fn ClosePockets
  (Variables|Default|SetbPocketsOpen false)
  (for _array_element (Variables|Default|GetOutOfPocketItems)
    (CallFunction|PutIteminPocket _array_element)))

(fn IsIteminPockets
  (params (Item :type I%20Pocket%20Item%20Interface))
  (return (and (CallFunction|DoPocketsContainItem Item) (not (Utilities|Array|ContainsItem (Variables|Default|GetOutOfPocketItems) Item)))))

(fn IsItemIndexinPockets
  (params (Index :type Integer))
  (if (Utilities|Array|IsValidIndex (Variables|Default|GetPocketItems) Index)
    (return (CallFunction|IsIteminPockets (Utilities|Array|Get(acopy) (Variables|Default|GetPocketItems) Index)))
    (else
      (return false))))