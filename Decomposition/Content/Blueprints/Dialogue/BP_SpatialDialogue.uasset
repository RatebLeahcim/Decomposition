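; BP_SpatialDialogue is a one-shot box trigger that advances an Inkpot story when an actor overlaps it.
; On overlap it prints a debug message, sends the "pickUp" path to ACStoryProvider with TestString as an Ink parameter, continues the story, then destroys itself.
; BeginPlay draws a temporary debug box showing the trigger's extent.
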(event Collision|EventActorBeginOverlap
  (params (OtherActor :type Actor%20Object%20Reference))
  (bind _ac_storyprovider (Variables|Default|GetAC_StoryProvider))
  (Development|PrintString "Hello" true true "(R=0.248858,G=0.000000,B=1.000000,A=1.000000)")
  (Class|BPIStoryProvider|ChoosePathParameter(Message) _ac_storyprovider "pickUp" (Utilities|Array|MakeArray (Class|InkpotLibrary|MakeStringInkpotValue (Variables|Default|GetTestString))))
  (Default|ContinueStory _ac_storyprovider)
  (Actor|DestroyActor))

(event EventBeginPlay
  (bind _box (Variables|Default|GetBox))
  (Rendering|Debug|DrawDebugBox (Transformation|GetWorldLocation _box) (Components|Box|GetScaledBoxExtent _box) "(R=0.376054,G=0.305122,B=1.000000,A=1.000000)" "0, 0, 0" 9e+01 5.0))

(fn ConstructionScript)