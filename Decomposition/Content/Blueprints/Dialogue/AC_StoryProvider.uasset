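; Actor component that provides an Inkpot (Ink) story to its story receivers for the game's dialogue.
; It registers itself with BP_FirstPersonGameMode on BeginPlay; Initialize binds to Inkpot's story-begin event and initializes each receiver with itself.
; It caches the story when it begins, then wraps continuing, choice selection and path jumps.
; A dispatcher relays when a path end is reached.
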(event EventBeginPlay
  (bind _asbp_first_person_game_mode (Utilities|Casting|CastToBP_FirstPersonGameMode (Game|GetGameMode)))
  (Utilities|Array|Add (Variables|/Game/Dynamic/FirstPerson/Blueprints/BP_FirstPersonGameMode.BP_FirstPersonGameMode_C|GetStoryProviders _asbp_first_person_game_mode) self))

(event EventTick
  (params (DeltaSeconds :type Float%20%28single-precision%29)))

(event EventOnStoryBegin
  (params (Story :type Inkpot%20Story%20Object%20Reference))
  (Variables|Default|SetStory Story))

(event EventInitialize
  (EventDispatchers|BindEventtoEventonStoryBegin (|Inkpot) (delegate EventOnStoryBegin))
  (for _array_element (Variables|Default|GetStoryReceivers)
    (Default|Initialize _array_element self)))

(event EventMakeChoice
  (params (Choice :type Inkpot%20Choice%20Object%20Reference))
  (Class|InkpotStory|ChooseChoice (Variables|Default|GetStory) Choice))

(event EventMakeChoiceIndex
  (params (ChoiceIndex :type Integer))
  (Class|InkpotStory|ChooseChoiceIndex (Variables|Default|GetStory) ChoiceIndex))

(event EventChoosePath
  (params (Path :type String))
  (Class|InkpotStory|ChoosePath (Variables|Default|GetStory) Path))

(event EventReachedPathEnd
  (Default|CallOnReachedPathEnd))

(fn ContinueStory
  (if (Class|InkpotStory|CanContinue (Variables|Default|GetStory))
    (Class|InkpotStory|Continue (Variables|Default|GetStory))
    (return true)
    (else
      (return false))))