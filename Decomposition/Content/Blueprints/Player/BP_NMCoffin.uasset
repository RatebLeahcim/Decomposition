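; Possessable coffin pawn that the player picks up, carries and drops, triggering Ink story lines on pickup and drop.
; Interaction walks the player to the coffin's foot, then possesses the coffin; Use or Drop teleports the character there and repossesses it.
; Movement steps a probe point projected onto the navmesh.
; Steering applies a clamped yaw offset that unwinds while moving, turning the controller when moving forward.
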(event InteractionEndEvent(AC_InteractionComponent)
  (params (Tool :type AC%20Tool%20Component%20Object%20Reference))
  ;[0.05098 0.05098 0.05098] Toggle picking up coffin
  (Variables|Default|SetTool Tool)
  (CallFunction|OnPickupCoffin))

(event Custom|StartPickUp
  (bind _footlocation (Variables|Default|GetFootLocation))
  (bind _returnvalue (Transformation|GetWorldLocation _footlocation))
  ;[0.05098 0.05098 0.05098] Update using cached rotation and movement logic
  (Input|SetIgnoreMoveInput (Game|GetPlayerController 0) true)
  (Utilities|FlowControl|Gate true) ; enters at Open
)

(event Custom|StopPickUp
  (bind _footlocation (Variables|Default|GetFootLocation))
  (bind _returnvalue (Transformation|GetWorldLocation _footlocation))
  ;[0.05098 0.05098 0.05098] Update using cached rotation and movement logic
  (Input|ResetIgnoreMoveInput (Game|GetPlayerController 0))
  (Utilities|FlowControl|Gate true) ; enters at Close
)

(event Input|EnhancedActionEvents|EnhancedInputActionIA_Move
  (params (ActionValue :type Vector%202D%20Structure) (ElapsedSeconds :type Float%20%28double-precision%29) (TriggeredSeconds :type Float%20%28double-precision%29) (InputAction :type Input%20Action%20Object%20Reference :default "/Game/Input/Actions/IA_Move.IA_Move"))
  ;[0.05098 0.05098 0.05098] Update and cache rotation
  (Variables|Default|SetRotationOffset (Math|Rotator|MakeRotator (.roll (Math|Rotator|CombineRotators (Variables|Default|GetRotationOffset) (Math|Rotator|MakeRotator 0.0 0.0 (* (.x ActionValue) (Variables|Settings|GetRotationSpeed) (Utilities|Time|GetWorldDeltaSeconds) (Variables|Settings|GetInvertControls))))) (.pitch (Math|Rotator|CombineRotators (Variables|Default|GetRotationOffset) (Math|Rotator|MakeRotator 0.0 0.0 (* (.x ActionValue) (Variables|Settings|GetRotationSpeed) (Utilities|Time|GetWorldDeltaSeconds) (Variables|Settings|GetInvertControls))))) (Math|Float|Clamp(Float) (.yaw (Math|Rotator|CombineRotators (Variables|Default|GetRotationOffset) (Math|Rotator|MakeRotator 0.0 0.0 (* (.x ActionValue) (Variables|Settings|GetRotationSpeed) (Utilities|Time|GetWorldDeltaSeconds) (Variables|Settings|GetInvertControls))))) -45.0 45.0)))
  (if (and (Utilities|Operators|NotEqual(!=) :A (Variables|Default|GetRotationOffset) :ErrorTolerance 0.3) (Utilities|IsMovingFB))
    (Variables|Default|SetRotationOffset (Math|Rotator|CombineRotators (Variables|Default|GetRotationOffset) (Math|Rotator|MakeRotator 0.0 0.0 (* (* (Math|Float|Sign(Float) (.yaw (Math|Rotator|CombineRotators (Variables|Default|GetRotationOffset) (Math|Rotator|MakeRotator 0.0 0.0 (* (.x ActionValue) (Variables|Settings|GetRotationSpeed) (Utilities|Time|GetWorldDeltaSeconds) (Variables|Settings|GetInvertControls)))))) -1.0) (Variables|Settings|GetRotationSpeed) (Utilities|Time|GetWorldDeltaSeconds) 0.3))))
    (if (Utilities|IsMovingForward)
      (Pawn|Input|AddControllerYawInput (* (* (* (Math|Float|Sign(Float) (.yaw (Math|Rotator|CombineRotators (Variables|Default|GetRotationOffset) (Math|Rotator|MakeRotator 0.0 0.0 (* (.x ActionValue) (Variables|Settings|GetRotationSpeed) (Utilities|Time|GetWorldDeltaSeconds) (Variables|Settings|GetInvertControls)))))) -1.0) (Variables|Settings|GetRotationSpeed) (Utilities|Time|GetWorldDeltaSeconds) 0.3) -1.0)))))

(event Input|EnhancedActionEvents|EnhancedInputActionIA_Drop
  (params (ActionValue :type Boolean) (ElapsedSeconds :type Float%20%28double-precision%29) (TriggeredSeconds :type Float%20%28double-precision%29) (InputAction :type Input%20Action%20Object%20Reference :default "/Game/Input/Actions/IA_Drop.IA_Drop"))
  ;[1 1 1] Handles "Use" or "Drop" - Switches Back to Player Pawn
  (:Completed
    (bind _outactors (Actor|GetAllActorsOfClass "/Game/Blueprints/Player/BP_PlayerCharacter.BP_PlayerCharacter_C"))
    (Transformation|SetActorTransform (Utilities|Array|Get(acopy) _outactors) (Transformation|GetWorldTransform (Variables|Default|GetFootLocation)) false true)
    (Pawn|Possess (Game|GetPlayerController 0) (Utilities|Array|Get(acopy) _outactors))
    (CallFunction|OnDropCoffin)))

(event Input|EnhancedActionEvents|EnhancedInputActionIA_Use
  (params (ActionValue :type Boolean) (ElapsedSeconds :type Float%20%28double-precision%29) (TriggeredSeconds :type Float%20%28double-precision%29) (InputAction :type Input%20Action%20Object%20Reference :default "/Game/Input/Actions/IA_Use.IA_Use"))
  ;[1 1 1] Handles "Use" or "Drop" - Switches Back to Player Pawn
  (:Completed
    (bind _outactors (Actor|GetAllActorsOfClass "/Game/Blueprints/Player/BP_PlayerCharacter.BP_PlayerCharacter_C"))
    (Transformation|SetActorTransform (Utilities|Array|Get(acopy) _outactors) (Transformation|GetWorldTransform (Variables|Default|GetFootLocation)) false true)
    (Pawn|Possess (Game|GetPlayerController 0) (Utilities|Array|Get(acopy) _outactors))
    (CallFunction|OnDropCoffin)))

(event EventBeginPlay
  (bind _returnvalue (Transformation|GetActorLocation))
  (CallFunction|AddIMC "/Game/Input/IMC_Default.IMC_Default")
  (CallFunction|Setup)
  ;[0.05098 0.05098 0.05098] PlayerHeight has been chosen to put the player at about the same height as the BP_PlayerCharacter pawn
  (Transformation|SetRelativeLocation (Variables|Default|GetMoveCheckLocation) (Math|Vector|MakeVector 4e+02 0.0 (* (Variables|Settings|GetPlayerHeight) -1.0)) false false)
  (Transformation|SetActorLocation (Math|Vector|MakeVector (.x _returnvalue) (.y _returnvalue) (Variables|Settings|GetPlayerHeight)) false false)
  (Input|EnableInput (Game|GetPlayerController 0))
  (bind _asbp_player_character (Utilities|Casting|CastToBP_PlayerCharacter (Game|GetPlayerCharacter 0)))
  (Variables|Default|SetPlayerReference _asbp_player_character)
  (Variables|Components|SetCoffin%20Carry%20Point (Variables|/Game/Blueprints/Player/BP_PlayerCharacter.BP_PlayerCharacter_C|GetCoffinCarryPoint _asbp_player_character)))

(event EventTick
  (params (DeltaSeconds :type Float%20%28single-precision%29))
  (bind _returnvalue (Utilities|Time|GetWorldDeltaSeconds))
  (bind _returnvalue_2 (Class|NavigationSystemV1|GetNavigationSystem))
  (bind _returnvalue_3 (Input|EnhancedActionValues|GetIA_Move))
  (bind _coffinspeed (Variables|Settings|GetCoffinSpeed))
  (bind _upright (Variables|Default|GetUpright))
  (bind _queryextent (Variables|Settings|GetQueryExtent))
  (bind _footlocation (Variables|Default|GetFootLocation))
  (bind _movechecklocation (Variables|Default|GetMoveCheckLocation))
  (bind _returnvalue_4 (Transformation|GetWorldLocation _footlocation))
  (bind _returnvalue_5 (Math|Vector|GetRightVector _upright))
  (bind _returnvalue_6 (Transformation|GetWorldLocation _movechecklocation))
  (bind _returnvalue_7 (* _returnvalue_5 (.y _returnvalue_3) _returnvalue _coffinspeed))
  (bind _returnvalue_8 (+ _returnvalue_6 _returnvalue_7))
  (bind (_projectedlocation _returnvalue_9) (AI|Navigation|ProjectPointtoNavigation _returnvalue_2 _returnvalue_8 0 0 _queryextent))
  ;[0.05098 0.05098 0.05098] Update using cached rotation and movement logic
  (Utilities|FlowControl|Sequence
    (:then_0
      (Utilities|FlowControl|Gate true
        (:Exit
          (Pawn|Input|AddMovementInput (Variables|Default|GetPlayerReference) (Math|Vector|Normalize (- (Transformation|GetWorldLocation (Variables|Default|GetFootLocation)) (Transformation|GetActorLocation (Variables|Default|GetPlayerReference)))) 2.0 true)
          (Input|EnableInput (Game|GetPlayerController 0))
          (bind _asbp_player_character (Utilities|Casting|CastToBP_PlayerCharacter (Game|GetPlayerCharacter 0)))
          (Variables|Default|SetPlayerReference _asbp_player_character)
          (Variables|Components|SetCoffin%20Carry%20Point (Variables|/Game/Blueprints/Player/BP_PlayerCharacter.BP_PlayerCharacter_C|GetCoffinCarryPoint _asbp_player_character))
          (Development|PrintString (Utilities|String|ToString(Vector) (Transformation|GetActorLocation (Variables|Default|GetPlayerReference))) true true "(R=0.056731,G=0.065059,B=1.000000,A=1.000000)" 6.0)
          (Development|PrintString (Utilities|String|ToString(Vector) _returnvalue_4) true true "(R=0.000000,G=0.582484,B=1.000000,A=1.000000)" 6.0)
          (if (Utilities|Operators|EqualEqual (Math|Conversions|ToVector2D(Vector) (Transformation|GetActorLocation (Variables|Default|GetPlayerReference))) (Math|Conversions|ToVector2D(Vector) _returnvalue_4) 0.1)
            (CallFunction|StopPickUp)
            (CallFunction|OnPickupFinished)))))
    (:then_1
      (Transformation|SetRelativeRotation (Variables|Default|GetUpright) (Math|Interpolation|RInterpTo (Variables|/Script/Engine.SceneComponent|GetRelativeRotation (Variables|Default|GetUpright)) (Math|Rotator|CombineRotators (Variables|Default|GetCoffinTargetRotation) (Variables|Default|GetRotationOffset)) DeltaSeconds 3e+01) false false)
      ;;[0.05098 0.05098 0.05098] Moving player character towards the coffin before picking it up should happen in the BP_PlayerCharacter blueprint now, since this BP can be considered more or less inactive until the pickup is complete
      (if (and _returnvalue_9 (Utilities|IsMovingFB))
        (Transformation|SetActorLocation (+ (+ _projectedlocation (- (Transformation|GetWorldLocation (Variables|Default|GetFootLocation)) (Transformation|GetWorldLocation (Variables|Default|GetMoveCheckLocation)))) (Math|Vector|MakeVector 0.0 0.0 (Variables|Settings|GetPlayerHeight))) false false)))))

(event EventOnSettingsChanged
  (params (Settings :type F%20Game%20Settings%20Structure))
  ;[0.05098 0.05098 0.05098] Load Save data
  (Variables|Settings|SetInvertControls (Math|Float|SelectFloat 1.0 -1.0 (.InvertControls (Utilities|Struct|BreakFGameSettings Settings)))))

(event Input|KeyboardEvents|DebugKeyEnd
  (params (Key :type Key%20Structure :default "None") (ActionValue :type Input%20Action%20Value%20Structure))
  ;[1 1 1] Debug Pawn Switch Key
  (:Pressed
    (bind _outactors (Actor|GetAllActorsOfClass "/Game/Blueprints/Player/BP_PlayerCharacter.BP_PlayerCharacter_C"))
    (Pawn|Possess (Game|GetPlayerController 0) (Utilities|Array|Get(acopy) _outactors))))

(fn ConstructionScript)

(fn Setup
  (Variables|/Game/Blueprints/Interaction/AC_InteractionComponent.AC_InteractionComponent_C|SetOutlineObjects (Variables|Default|GetAC_InteractionComponent) (Utilities|Array|MakeArray (Variables|Default|GetUpright))))

(fn AddIMC
  (params (Mapping%20Context :type Input%20Mapping%20Context%20Object%20Reference))
  (bind _asplayer_controller (Utilities|Casting|CastToPlayerController (Pawn|GetController)))
  (Utilities|IsValid (PlayerController|LocalPlayerSubsystems|GetEnhancedInputLocalPlayerSubsystem _asplayer_controller)
    (:Is%20Valid
      (Input|AddMappingContext (PlayerController|LocalPlayerSubsystems|GetEnhancedInputLocalPlayerSubsystem _asplayer_controller) Mapping%20Context 0 "(bIgnoreAllPressedKeysUntilRelease=True,bForceImmediately=False,bNotifyUserSettings=False)"))))

(fn UserConstructionScript0
  (Variables|/Game/Blueprints/Interaction/AC_InteractionComponent.AC_InteractionComponent_C|SetOutlineObjects (Variables|Default|GetAC_InteractionComponent) (Utilities|Array|MakeArray (Variables|Default|GetUpright))))

(fn OnPickupCoffin
  (bind _tool (Variables|Default|GetTool))
  (bind _pockets (Variables|/Game/Blueprints/Interaction/AC_ToolComponent.AC_ToolComponent_C|GetPockets _tool))
  (Default|HideInteractionUI _tool)
  (Utilities|IsValid _pockets
    (:Is%20Valid
      (Default|ClosePockets _pockets))
    (:Is%20Not%20Valid
      _))
  (CallFunction|StartPickUp)
  (Default|HoldInteractable _tool (Variables|Default|GetAC_InteractionComponent))
  (Default|DisableInteraction (Variables|Default|GetAC_InteractionComponent)))

(fn OnDropCoffin
  (bind _ac_storyprovider (Variables|Default|GetAC_StoryProvider))
  (bind _tool (Variables|Default|GetTool))
  (bind _pockets (Variables|/Game/Blueprints/Interaction/AC_ToolComponent.AC_ToolComponent_C|GetPockets _tool))
  (Variables|Default|SetOffset "0, 0, 0")
  (Default|SetToolMode (Variables|Default|GetTool) "NewEnumerator0")
  (Class|BPIGrabber|OnDropped(Message) (Game|GetPlayerCharacter 0) "Coffin")
  (Utilities|IsValid _pockets
    (:Is%20Valid
      (Default|OpenPockets _pockets))
    (:Is%20Not%20Valid
      _))
  (Default|EnableInteraction (Variables|Default|GetAC_InteractionComponent))
  (Collision|SetCollisionResponsetoChannel (Variables|Default|GetUpright) "ECC_GameTraceChannel3" "ECR_Block")
  (Default|ChoosePathParameter _ac_storyprovider "onDropCoffin" (Utilities|Array|MakeArray (Class|InkpotLibrary|MakeIntInkpotValue (Math|Random|RandomIntegerinRange 0 2))))
  (Default|ContinueStory _ac_storyprovider)
  (Collision|SetCollisionResponsetoChannel (Variables|Default|GetUpright) "ECC_GameTraceChannel4" "ECR_Overlap"))

(fn OnPickupFinished
  (bind _ac_storyprovider (Variables|Default|GetAC_StoryProvider))
  (Development|PrintString "pickup finished?" true true "(R=0.606574,G=0.000000,B=1.000000,A=1.000000)" 1e+01)
  (Default|SetToolMode (Variables|Default|GetTool) "NewEnumerator2")
  (Class|BPIGrabber|OnGrabbed(Message) (Game|GetPlayerCharacter 0) "Coffin" self)
  (Variables|Default|SetbIsPickedUp true)
  (Collision|SetCollisionResponsetoChannel (Variables|Default|GetUpright) "ECC_GameTraceChannel3" "ECR_Ignore")
  (Development|PrintString "before possess")
  (bind _outactors (Actor|GetAllActorsOfClass "BP_NMCoffin_C"))
  (Pawn|Possess (Game|GetPlayerController 0) (Utilities|Array|Get(acopy) _outactors))
  (Development|PrintString "after posses")
  (Default|ChoosePathParameter _ac_storyprovider "onPickUpCoffin" (Utilities|Array|MakeArray (Class|InkpotLibrary|MakeIntInkpotValue (Math|Random|RandomIntegerinRange 0 4))))
  (Default|ContinueStory _ac_storyprovider)
  (Collision|SetCollisionResponsetoChannel (Variables|Default|GetUpright) "ECC_GameTraceChannel4" "ECR_Ignore"))