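; BP_WallLantern is a wall lantern prop whose point light flickers on at BeginPlay or when the player first overlaps its trigger, depending on flags.
; The FlickerOn timeline curve scales maximum intensity, optionally looping forward from a fixed later time after random delays.
; The construction script can show a separate editor preview intensity.
; A debug numpad key reverses the timeline to flicker the light off.
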(event OnComponentBeginOverlap(FlickerOnTrigger)
  (params (OverlappedComponent :type Primitive%20Component%20Object%20Reference) (OtherActor :type Actor%20Object%20Reference) (OtherComp :type Primitive%20Component%20Object%20Reference) (OtherBodyIndex :type Integer) (bFromSweep :type Boolean) (SweepResult :type Hit%20Result%20Structure%20%28by%20ref%29))
  (if (and (== OtherActor (Game|Player|GetPlayerPawn 0)) (Variables|Default|GetbFlickerOnTrigger))
    (CallFunction|FlickerLighton)
    (Variables|Default|SetbFlickerOnTrigger false)))

(event Custom|FlickerLightOn
  (bind (_direction _lightoncurve) (Timeline|FlickerOn PlayFromStart)
    (:Update
      (CallFunction|SetLightIntensity _lightoncurve (Variables|Default|GetMaxLightIntensity)))
    (:Finished
      (if (Variables|Default|GetbLoopFlicker)
        (switch Utilities|FlowControl|Switch|SwitchonETimelineDirection _direction
          (:Forward
            (Utilities|FlowControl|Delay (Math|Random|RandomFloatinRange 0.0 (Variables|Default|GetMaxFlickerDelay)))
            (CallFunction|SetNewTime 0.42)
            (CallFunction|FlickerCurrent)))))))

(event Custom|FlickerLightOff
  (bind (_direction _lightoncurve) (Timeline|FlickerOn ReverseFromEnd)
    (:Update
      (CallFunction|SetLightIntensity _lightoncurve (Variables|Default|GetMaxLightIntensity)))
    (:Finished
      (if (Variables|Default|GetbLoopFlicker)
        (switch Utilities|FlowControl|Switch|SwitchonETimelineDirection _direction
          (:Forward
            (Utilities|FlowControl|Delay (Math|Random|RandomFloatinRange 0.0 (Variables|Default|GetMaxFlickerDelay)))
            (CallFunction|SetNewTime 0.42)
            (CallFunction|FlickerCurrent)))))))

(event Custom|SetNewTime
  (params (Time :type Float%20%28double-precision%29))
  (bind (_direction _lightoncurve) (Timeline|FlickerOn SetNewTime)
    (:Update
      (CallFunction|SetLightIntensity _lightoncurve (Variables|Default|GetMaxLightIntensity)))
    (:Finished
      (if (Variables|Default|GetbLoopFlicker)
        (switch Utilities|FlowControl|Switch|SwitchonETimelineDirection _direction
          (:Forward
            (Utilities|FlowControl|Delay (Math|Random|RandomFloatinRange 0.0 (Variables|Default|GetMaxFlickerDelay)))
            (CallFunction|SetNewTime 0.42)
            (CallFunction|FlickerCurrent)))))))

(event Custom|FlickerCurrent
  (bind (_direction _lightoncurve) (Timeline|FlickerOn Play)
    (:Update
      (CallFunction|SetLightIntensity _lightoncurve (Variables|Default|GetMaxLightIntensity)))
    (:Finished
      (if (Variables|Default|GetbLoopFlicker)
        (switch Utilities|FlowControl|Switch|SwitchonETimelineDirection _direction
          (:Forward
            (Utilities|FlowControl|Delay (Math|Random|RandomFloatinRange 0.0 (Variables|Default|GetMaxFlickerDelay)))
            (CallFunction|SetNewTime 0.42)
            (CallFunction|FlickerCurrent)))))))

(event EventBeginPlay
  (Utilities|FlowControl|Sequence
    (:then_0
      (Input|EnableInput (Game|GetPlayerController 0))
      (Rendering|Components|Light|SetIntensity (Variables|Default|GetPointLight) (Variables|Default|GetLightIntensity)))
    (:then_1
      (if (Variables|Default|GetbFlickerOnPlay)
        (CallFunction|FlickerLighton)))
    (:then_2
      (if (not (Variables|Default|GetbFlickerOnTrigger))
        (Components|Activation|SetActive (Variables|Default|GetFlickerOnTrigger) false false)))))

(event Input|KeyboardEvents|DebugKeyNumPadZero
  (params (Key :type Key%20Structure :default "None") (ActionValue :type Input%20Action%20Value%20Structure))
  (:Pressed
    (CallFunction|FlickerLightOff)))

(fn ConstructionScript
  (Rendering|Components|Light|SetIntensity (Variables|Default|GetPointLight) (Math|Float|SelectFloat (Variables|Default|GetEditorIntensity) (Variables|Default|GetLightIntensity) (Variables|Default|GetbShowLightInEditor))))

(fn SetLightIntensity
  (params (IntensityPercentage :type Float%20%28double-precision%29) (MaxIntensity :type Float%20%28double-precision%29))
  (Rendering|Components|Light|SetIntensity (Variables|Default|GetPointLight) (* IntensityPercentage MaxIntensity)))