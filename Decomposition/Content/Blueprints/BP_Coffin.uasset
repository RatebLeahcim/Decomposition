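; Coffin the player picks up, drags and drops through an interaction component, with drag audio and random Ink story lines on pickup and drop.
; Pickup auto-walks the player to an attach point, then grabs the model with a physics handle.
; Each tick sweeps toward the target transform, reverts, then drives the handle there or slides along blocking walls.
; Player movement holds based on coffin roll and clear paths; step-up logic is disconnected.
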(event UseItemEvent(AC_InteractionComponent)
  (params (Tool :type AC%20Tool%20Component%20Object%20Reference))
  ;[0.05098 0.05098 0.05098] Since coffin is a held item, Use is called when Interact is pressed while holding it, which will call DropItem
  (Default|DropInteractable Tool))

(event InteractionEndEvent(AC_InteractionComponent)
  (params (Tool :type AC%20Tool%20Component%20Object%20Reference))
  ;[0.05098 0.05098 0.05098] Toggle picking up coffin
  (Variables|Default|SetTool Tool)
  (CallFunction|OnPickupCoffin))

(event DropEvent(AC_InteractionComponent)
  (params (Tool :type AC%20Tool%20Component%20Object%20Reference))
  ;[0.05098 0.05098 0.05098] Since coffin is a held item, Use is called when Interact is pressed while holding it, which will call DropItem
  (if (Variables|Default|GetbIsPickedUp)
    (Variables|Default|SetbIsPickedUp false)
    (CallFunction|OnDropCoffin)))

(event Custom|StartPickUp
  (bind _playerreference (Variables|Default|GetPlayerReference))
  ;[0.05098 0.05098 0.05098] Move player towards coffin when picked up
  (Input|SetIgnoreMoveInput (Game|GetPlayerController 0) true)
  (Utilities|FlowControl|Gate true) ; enters at Open
)

(event Custom|StopPickUp
  (bind _playerreference (Variables|Default|GetPlayerReference))
  ;[0.05098 0.05098 0.05098] Move player towards coffin when picked up
  (Input|ResetIgnoreMoveInput (Game|GetPlayerController 0))
  (Utilities|FlowControl|Gate true) ; enters at Close
)

(event Custom|AllowDragginEvent
  ;[0.05098 0.05098 0.05098] Play Sounds
  (Utilities|FlowControl|DoOnce false) ; enters at Reset
)

(event Input|EnhancedActionEvents|EnhancedInputActionIA_Move
  (params (ActionValue :type Vector%202D%20Structure) (ElapsedSeconds :type Float%20%28double-precision%29) (TriggeredSeconds :type Float%20%28double-precision%29) (InputAction :type Input%20Action%20Object%20Reference :default "/Game/Input/Actions/IA_Move.IA_Move"))
  ;[0.05098 0.05098 0.05098] Play Sounds
  (:Triggered
    (if (and (Variables|Default|GetbIsPickedUp) (Utilities|Operators|NotEqual(!=) :A (Transformation|GetVelocity (Game|GetPlayerCharacter 0))))
      (Utilities|FlowControl|DoOnce false
        (:Completed
          (bind _returnvalue (Class|FMODBlueprintStatics|PlayEvent2D "/Game/FMOD/Events/SFX/PlayerInteractionSFX/CoffinDraggingMAIN.CoffinDraggingMAIN"))
          (Variables|Default|SetDraggingSoundEvent _returnvalue)))
      (else
        (Class|FMODBlueprintStatics|EventInstanceStop (Variables|Default|GetDraggingSoundEvent) false))))
  (:Canceled
    (Class|FMODBlueprintStatics|EventInstanceStop (Variables|Default|GetDraggingSoundEvent) false :!label _label)
    (CallFunction|AllowDragginEvent))
  (:Completed
    (goto _label)))

(event EventBeginPlay
  (Input|EnableInput (Game|GetPlayerController 0))
  (bind _asbp_player_character (Utilities|Casting|CastToBP_PlayerCharacter (Game|GetPlayerCharacter 0)))
  (Variables|Default|SetPlayerReference _asbp_player_character)
  (Variables|Default|SetCoffin%20Carry%20Point (Variables|/Game/Blueprints/Player/BP_PlayerCharacter.BP_PlayerCharacter_C|GetCoffinCarryPoint _asbp_player_character)))

(event Collision|EventActorBeginOverlap
  (params (OtherActor :type Actor%20Object%20Reference)))

(event EventTick
  (params (DeltaSeconds :type Float%20%28single-precision%29))
  (bind _returnvalue (Transformation|GetActorLocation))
  (bind (_targetlocation _targetrotation) (Utilities|TargetTransform))
  (bind _physics_handle (Variables|Default|GetPhysics%20Handle))
  (bind _playerreference (Variables|Default|GetPlayerReference))
  (bind _playerreference_2 (Variables|Default|GetPlayerReference))
  ;[0.05098 0.05098 0.05098] Move player towards coffin when picked up
  (Utilities|FlowControl|Sequence
    (:then_0
      (Utilities|FlowControl|Gate true
        (:Exit
          (Pawn|Input|AddMovementInput _playerreference_2 (Math|Vector|Normalize (- (Transformation|GetWorldLocation (Variables|Default|GetPlayerAttachPoint)) (Transformation|GetActorLocation _playerreference_2))) 2.0 true)
          (if (Utilities|Operators|EqualEqual (Math|Conversions|ToVector2D(Vector) (Transformation|GetActorLocation (Variables|Default|GetPlayerReference))) (Math|Conversions|ToVector2D(Vector) (Transformation|GetWorldLocation (Variables|Default|GetPlayerAttachPoint))) 0.1)
            (CallFunction|StopPickUp)
            (CallFunction|OnPickupFinished)))))
    (:then_1
      (if (Variables|Default|GetbIsPickedUp)
        (Variables|Default|SetCurrentLocation (Transformation|GetActorLocation))
        (Variables|Default|SetCurrentRotation (Transformation|GetActorRotation))
        (bind _sweephitresult (Transformation|SetActorLocationAndRotation _targetlocation _targetrotation true)) ; Check if the location we're trying to move to has any collisions along the way
        (Transformation|SetActorLocationAndRotation (Variables|Default|GetCurrentLocation) (Variables|Default|GetCurrentRotation) false true) ; Undo movement from that previous check - we want the physics handle to move us
        (if (.bBlockingHit (Collision|BreakHitResult _sweephitresult)) ; Only move if the path was clear
          (if (!= (.y (Input|EnhancedActionValues|GetIA_Move)) 0.0)
            (Class|PhysicsHandleComponent|SetTargetLocationandRotation _physics_handle (Math|Interpolation|VInterpTo _returnvalue (+ (CallFunction|GetSlidingLocation (.ImpactPoint (Collision|BreakHitResult _sweephitresult)) (.ImpactNormal (Collision|BreakHitResult _sweephitresult))) (- (.Location (Collision|BreakHitResult _sweephitresult)) (.ImpactPoint (Collision|BreakHitResult _sweephitresult)))) DeltaSeconds 3e+01) (Math|Rotator|CombineRotators _targetrotation (Variables|Default|GetOffset)))
            (Variables|Default|SetOffset "0, 0, 0"))
          (else
            (Class|PhysicsHandleComponent|SetTargetLocationandRotation _physics_handle (Math|Interpolation|VInterpTo _returnvalue _targetlocation DeltaSeconds 3e+01) (Math|Rotator|CombineRotators _targetrotation (Variables|Default|GetOffset)))
            (Variables|/Game/Blueprints/Player/BP_PlayerCharacter.BP_PlayerCharacter_C|SetbHoldMovement (Variables|Default|GetPlayerReference) false)))))
    (:then_2
      (if (and (Variables|Default|GetbIsPickedUp) (Math|Float|NearlyEqual(Float) (.roll (Transformation|GetActorRotation)) 22.0 3.0))
        (Variables|/Game/Blueprints/Player/BP_PlayerCharacter.BP_PlayerCharacter_C|SetbHoldMovement _playerreference false)
        (else
          (Variables|/Game/Blueprints/Player/BP_PlayerCharacter.BP_PlayerCharacter_C|SetbHoldMovement _playerreference true))))))

(fn ConstructionScript
  (Variables|/Game/Blueprints/Interaction/AC_InteractionComponent.AC_InteractionComponent_C|SetOutlineObjects (Variables|Default|GetAC_InteractionComponent) (Utilities|Array|MakeArray (Variables|Default|GetModel))))

(fn OnPickupCoffin
  (bind _tool (Variables|Default|GetTool))
  (bind _pockets (Variables|/Game/Blueprints/Interaction/AC_ToolComponent.AC_ToolComponent_C|GetPockets _tool))
  (Default|HideInteractionUI _tool)
  (Utilities|IsValid _pockets
    (:Is%20Valid
      (Default|ClosePockets _pockets))
    (:Is%20Not%20Valid
      _))
  (CallFunction|StartPickUp)
  (Default|HoldInteractable _tool (Variables|Default|GetAC_InteractionComponent))
  (Default|DisableInteraction (Variables|Default|GetAC_InteractionComponent)))

(fn OnDropCoffin
  (bind _ac_storyprovider (Variables|Default|GetAC_StoryProvider))
  (bind _tool (Variables|Default|GetTool))
  (bind _pockets (Variables|/Game/Blueprints/Interaction/AC_ToolComponent.AC_ToolComponent_C|GetPockets _tool))
  (Variables|Default|SetOffset "0, 0, 0")
  (Default|SetToolMode (Variables|Default|GetTool) "NewEnumerator0")
  (Class|BPIGrabber|OnDropped(Message) (Game|GetPlayerCharacter 0) "Coffin")
  (Utilities|IsValid _pockets
    (:Is%20Valid
      (Default|OpenPockets _pockets))
    (:Is%20Not%20Valid
      _))
  (Default|EnableInteraction (Variables|Default|GetAC_InteractionComponent))
  (Collision|SetCollisionResponsetoChannel (Variables|Default|GetModel) "ECC_GameTraceChannel3" "ECR_Block")
  (Default|ChoosePathParameter _ac_storyprovider "onDropCoffin" (Utilities|Array|MakeArray (Class|InkpotLibrary|MakeIntInkpotValue (Math|Random|RandomIntegerinRange 0 2))))
  (Default|ContinueStory _ac_storyprovider)
  (Collision|SetCollisionResponsetoChannel (Variables|Default|GetModel) "ECC_GameTraceChannel4" "ECR_Overlap"))

(fn OnPickupFinished
  (bind _returnvalue (Game|GetPlayerCharacter 0))
  (bind _ac_storyprovider (Variables|Default|GetAC_StoryProvider))
  (bind _model (Variables|Default|GetModel))
  (Default|SetToolMode (Variables|Default|GetTool) "NewEnumerator2")
  (bind _physicshandle (Class|BPIGrabber|PickUpObject(Message) _returnvalue _model (Transformation|GetWorldLocation _model) (Math|Rotator|CombineRotators (Variables|/Script/Engine.SceneComponent|GetRelativeRotation _model) "0.000000,-90.000000,0.000000")))
  (Utilities|IsValid _physicshandle
    (:Is%20Valid
      (Variables|Default|SetPhysics%20Handle _physicshandle)
      (Class|BPIGrabber|OnGrabbed(Message) _returnvalue "Coffin" self)
      (Variables|Default|SetbIsPickedUp true)
      (Collision|SetCollisionResponsetoChannel (Variables|Default|GetModel) "ECC_GameTraceChannel3" "ECR_Ignore")
      (Default|ChoosePathParameter _ac_storyprovider "onPickUpCoffin" (Utilities|Array|MakeArray (Class|InkpotLibrary|MakeIntInkpotValue (Math|Random|RandomIntegerinRange 0 4))))
      (Default|ContinueStory _ac_storyprovider)
      (Collision|SetCollisionResponsetoChannel (Variables|Default|GetModel) "ECC_GameTraceChannel4" "ECR_Ignore"))
    (:Is%20Not%20Valid
      (Development|PrintString "Player is not a grabber!"))))

(fn TestforSteppableSurface
  (params (TraceComponent :type Scene%20Component%20Object%20Reference))
  (bind _returnvalue (Transformation|GetWorldLocation TraceComponent))
  (bind (_outhit _returnvalue_2) (Collision|LineTraceForObjects _returnvalue (+ _returnvalue (* (Math|Vector|GetForwardVector TraceComponent) (Variables|Default|GetTraceDistance))) (Utilities|Array|MakeArray "ObjectTypeQuery1" "ObjectTypeQuery2") false 0 "ForDuration"))
  (if _returnvalue_2
    (Rendering|Debug|DrawDebugLine (.ImpactPoint (Collision|BreakHitResult _outhit)) (+ (.ImpactPoint (Collision|BreakHitResult _outhit)) (* (.ImpactNormal (Collision|BreakHitResult _outhit)) 5e+01)) "(R=1.000000,G=0.937618,B=0.000000,A=1.000000)" 5.0 1.0)
    (if (and (== (Math|Vector|DotProduct (.ImpactNormal (Collision|BreakHitResult _outhit)) "0.000000,0.000000,1.000000") 1.0) (<= (Math|Float|Absolute(Float) (- (.Z (Math|Vector|BreakVector (.Location (Collision|BreakHitResult _outhit)))) (.z (Transformation|GetWorldLocation (Variables|Default|GetGroundLevel))))) (Variables|Default|GetStepUpMaxHeight)))
      (return true (Math|Float|Absolute(Float) (- (.Z (Math|Vector|BreakVector (.Location (Collision|BreakHitResult _outhit)))) (.z (Transformation|GetWorldLocation (Variables|Default|GetGroundLevel))))) "NewEnumerator0")
      (else
        (return false 0.0 "NewEnumerator1")))
    (else
      (return false 0.0 "NewEnumerator2"))))

(fn EvaluateTestResults
  (params (Results :type Array%20of%20E_CoffinTestResult%20Enums :default "NewEnumerator0"))
  (for _array_element Results
    (switch Utilities|FlowControl|Switch|SwitchonE_CoffinTestResult _array_element
      (:NewEnumerator0
        (Math|Integer|IncrementInt (LocalVariables|GetValidResults)))
      (:NewEnumerator1
        (Math|Integer|IncrementInt (LocalVariables|GetInvalidResults) :!label _label))
      (:NewEnumerator2
        (goto _label))))
  (return (> (LocalVariables|GetValidResults) (LocalVariables|GetInvalidResults))))

(fn CheckShouldPlaySounds
  (if (Utilities|Operators|EqualEqual :A (Transformation|GetVelocity))
    (Class|FMODBlueprintStatics|EventInstanceStop (Variables|Default|GetDraggingSoundEvent) false)
    (CallFunction|AllowDragginEvent)))

(fn GetSlidingLocation
  (params (HitPoint :type Vector) (HitNormal :type Vector))
  (bind _returnvalue (Input|EnhancedActionValues|GetIA_Move))
  (bind _playerreference (Variables|Default|GetPlayerReference))
  (bind _returnvalue_2 (Math|Vector|Normalize HitNormal))
  (bind _returnvalue_3 (Transformation|GetActorForwardVector _playerreference))
  (bind _returnvalue_4 (Math|Vector|CrossProduct _returnvalue_2 "0.000000,0.000000,1.000000"))
  (bind _returnvalue_5 (Math|Vector|NegateVector _returnvalue_4))
  (Rendering|Debug|DrawDebugPoint :Position HitPoint :Size 5.0 :Duration 1e+01)
  (Utilities|FlowControl|Sequence
    (:then_0
      (if (> (.y _returnvalue) 0.0)
        (LocalVariables|SetMovingForwards true)
        (elif (< (.y _returnvalue) 0.0)
          (LocalVariables|SetMovingForwards false))))
    (:then_1
      (Rendering|Debug|DrawDebugPoint (+ HitPoint (* (Math|Vector|SelectVector _returnvalue_4 _returnvalue_5 (> (Math|Vector|DotProduct _returnvalue_4 (Math|Vector|SelectVector _returnvalue_3 (Math|Vector|NegateVector _returnvalue_3) (LocalVariables|GetMovingForwards))) (Math|Vector|DotProduct _returnvalue_5 (Math|Vector|SelectVector _returnvalue_3 (Math|Vector|NegateVector _returnvalue_3) (LocalVariables|GetMovingForwards))))) 5.0)) 5.0 "(R=1.000000,G=0.011539,B=0.000000,A=1.000000)" 1e+01)
      (return (+ HitPoint (* (Math|Vector|SelectVector _returnvalue_4 _returnvalue_5 (> (Math|Vector|DotProduct _returnvalue_4 (Math|Vector|SelectVector _returnvalue_3 (Math|Vector|NegateVector _returnvalue_3) (LocalVariables|GetMovingForwards))) (Math|Vector|DotProduct _returnvalue_5 (Math|Vector|SelectVector _returnvalue_3 (Math|Vector|NegateVector _returnvalue_3) (LocalVariables|GetMovingForwards))))) 5.0))))))

(fn HasAllMatchingTags
  (params (TagContainer :type Gameplay%20Tag%20Container%20Structure))
  (return (GameplayTags|HasAllTags (Variables|Default|GetTagContainer) TagContainer true)))

(fn HasAnyMatchingTags
  (params (Tags :type Gameplay%20Tag%20Container%20Structure))
  (return (GameplayTags|HasAnyTags (Variables|Default|GetTagContainer) Tags)))

(fn HasMatchingTag
  (params (Tag :type Gameplay%20Tag%20Structure))
  (return (GameplayTags|HasTag (Variables|Default|GetTagContainer) Tag true)))