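; Speakeasy door actor that opens and closes by hiding its mesh and toggling collision, with FMOD door sounds.
; Each change passes a closed-state flag to a child spatial dialogue trigger, which is set to destroy on overlap while open.
; Opening also advances the Inkpot story along the door-activation path.
; A two-second cooldown gates the whole open or close action, not just the sounds, and EndPlay stops the closing sound.
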(event Custom|WaitToRe-enable
  (Utilities|FlowControl|Delay 2.0)
  (Variables|Default|SetbShouldPlaySounds true))

(event EventBeginPlay
  (bind _asbp_spatial_dialogue (Utilities|Casting|CastToBP_SpatialDialogue (Variables|/Script/Engine.ChildActorComponent|GetChildActor (Variables|Default|GetDialogueTrigger))))
  (Variables|/Game/Blueprints/Dialogue/BP_SpatialDialogue.BP_SpatialDialogue_C|SetParameters _asbp_spatial_dialogue (Utilities|Array|MakeArray (Class|InkpotLibrary|MakeBoolInkpotValue true))))

(event Collision|EventActorBeginOverlap
  (params (OtherActor :type Actor%20Object%20Reference)))

(event EventTick
  (params (DeltaSeconds :type Float%20%28single-precision%29)))

(event EventEndPlay
  (params (EndPlayReason :type EEndPlayReason%20Enum :default "Destroyed"))
  (Class|FMODBlueprintStatics|EventInstanceStop (Variables|Default|GetCloseEvent) false))

(fn ConstructionScript)

(fn OnDoorOpened
  (bind _ac_storyprovider (Variables|Default|GetAC_StoryProvider))
  (if (Variables|Default|GetbShouldPlaySounds)
    (bind _returnvalue (Class|FMODBlueprintStatics|PlayEvent2D "/Game/FMOD/Events/SFX/PlayerInteractionSFX/DoorOpen/DoorOpen.DoorOpen"))
    (Class|FMODBlueprintStatics|EventInstanceSetParameter _returnvalue "DoorOpen" 0.0)
    (Variables|Default|SetbShouldPlaySounds false)
    (bind _asbp_spatial_dialogue (Utilities|Casting|CastToBP_SpatialDialogue (Variables|/Script/Engine.ChildActorComponent|GetChildActor (Variables|Default|GetDialogueTrigger)))
      (:then
        (Variables|/Game/Blueprints/Dialogue/BP_SpatialDialogue.BP_SpatialDialogue_C|SetDestroyOnOverlap _asbp_spatial_dialogue true)
        (Variables|/Game/Blueprints/Dialogue/BP_SpatialDialogue.BP_SpatialDialogue_C|SetParameters _asbp_spatial_dialogue (Utilities|Array|MakeArray (Class|InkpotLibrary|MakeBoolInkpotValue false))))
      (:CastFailed
        _))
    (Collision|SetCollisionEnabled (Variables|Default|GetMesh) "NoCollision")
    (Development|SetHiddeninGame (Variables|Default|GetMesh) true false)
    (Default|ChoosePath _ac_storyprovider "onActivateDoor")
    (Default|ContinueStory _ac_storyprovider)
    (CallFunction|WaittoRe-enable)))

(fn OnDoorClosed
  (if (Variables|Default|GetbShouldPlaySounds)
    (bind _returnvalue (Class|FMODBlueprintStatics|PlayEvent2D "/Game/FMOD/Events/SFX/PlayerInteractionSFX/DoorOpen/DoorOpen.DoorOpen"))
    (bind _output_get (Variables|Default|SetCloseEvent _returnvalue))
    (Class|FMODBlueprintStatics|EventInstanceSetParameter _output_get "DoorOpen" 2.0)
    (Variables|Default|SetbShouldPlaySounds false)
    (bind _asbp_spatial_dialogue (Utilities|Casting|CastToBP_SpatialDialogue (Variables|/Script/Engine.ChildActorComponent|GetChildActor (Variables|Default|GetDialogueTrigger)))
      (:then
        (Variables|/Game/Blueprints/Dialogue/BP_SpatialDialogue.BP_SpatialDialogue_C|SetDestroyOnOverlap _asbp_spatial_dialogue false)
        (Variables|/Game/Blueprints/Dialogue/BP_SpatialDialogue.BP_SpatialDialogue_C|SetParameters _asbp_spatial_dialogue (Utilities|Array|MakeArray (Class|InkpotLibrary|MakeBoolInkpotValue true))))
      (:CastFailed
        _))
    (Collision|SetCollisionEnabled (Variables|Default|GetMesh) "QueryAndPhysics")
    (Development|SetHiddeninGame (Variables|Default|GetMesh) false false)
    (CallFunction|WaittoRe-enable)))