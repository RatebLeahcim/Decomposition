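; SP_EnemyAI is an enemy Blueprint that pursues the player and deals damage on contact.
; The FollowPlayer event moves it toward the player, and PawnSensing sends it to a seen pawn's location, both gated by Move.
; With Move off, a sighting issues a move to its own capsule location with no Pawn specified.
; Capsule hits against the player apply fixed damage.
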(event OnSeePawn(PawnSensing)
  (params (Pawn :type Pawn%20Object%20Reference))
  (if (Variables|Default|GetMove)
    (AI|AIMoveTo self (Transformation|GetActorLocation Pawn) 0 2e+01 false)
    (else
      (AI|AIMoveTo 0 (Transformation|GetWorldLocation (Variables|Collision|GetCapsuleComponent self)) 0 2e+01 false))))

(event OnComponentHit(CapsuleComponent)
  (params (HitComponent :type Primitive%20Component%20Object%20Reference) (OtherActor :type Actor%20Object%20Reference) (OtherComp :type Primitive%20Component%20Object%20Reference) (NormalImpulse :type Vector :default "0, 0, 0") (Hit :type Hit%20Result%20Structure%20%28by%20ref%29))
  (if (== OtherActor (Game|GetPlayerCharacter 0))
    (Game|Damage|ApplyDamage (Game|GetPlayerCharacter 0) 3e+01 0 0)))

(event Custom|Follow%20Player
  (params (F :type Key%20Structure :default "None"))
  (if (Variables|Default|GetMove)
    (AI|AIMoveTo self "0, 0, 0" (Game|GetPlayerCharacter 0) 5.0 false)))

(fn ConstructionScript)