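; BP_PatrolPath is a spline-based patrol route actor, placed in a monster AI test folder.
; PathProgression steps PathIndex by Direction and flips Direction at the first and last spline points, so the route runs back and forth rather than looping.
; GetSplinePointAsWorldPosition returns the world location of the current point on the PatrolPath spline.
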(event Custom|PathProgression
  (bind _output_get (Variables|Default|SetPathIndex (+ (Variables|Default|GetPathIndex) (Variables|Default|GetDirection))))
  (if (== _output_get (- (Spline|GetNumberOfSplinePoints (Variables|Default|GetPatrolPath)) 1))
    (Variables|Default|SetDirection -1)
    (elif (== 0 (Variables|Default|GetPathIndex))
      (Variables|Default|SetDirection 1))))

(fn ConstructionScript)

(fn GetSplinePointasWorldPosition
  (return (Spline|GetLocationatSplinePoint (Variables|Default|GetPatrolPath) (Variables|Default|GetPathIndex) "World")))