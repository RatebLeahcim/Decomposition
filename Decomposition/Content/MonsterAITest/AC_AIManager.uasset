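; AI manager component that splits the level's patrol points into patrol groups, apparently for monster AI.
; On BeginPlay it gathers every BP_PatrolPoint actor, assigns them alternately to two groups with a FlipFlop, and stores the array.
; The split follows array order, with no spatial or priority sorting.
; GetPatrolPoints filters a supplied array and returns the points matching a requested group.
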(event EventBeginPlay
  (bind _outactors (Actor|GetAllActorsOfClass "/Game/MonsterAITest/BP_PatrolPoint.BP_PatrolPoint_C"))
  (bind _sortedpatrolpoints (CallFunction|SortPatrolPoints _outactors))
  (Variables|Default|SetSortedPatrolPoints _sortedpatrolpoints))

(event EventTick
  (params (DeltaSeconds :type Float%20%28single-precision%29)))

(fn SortPatrolPoints
  (params (PatrolPoints :type Array%20of%20BP%20Patrol%20Point%20Object%20References))
  (for _array_element PatrolPoints
    (bind _asbp_patrol_point (Utilities|Casting|CastToBP_PatrolPoint _array_element))
    (Utilities|FlowControl|FlipFlop
      (:A
        (Variables|/Game/MonsterAITest/BP_PatrolPoint.BP_PatrolPoint_C|SetE_PatrolGroup _asbp_patrol_point "NewEnumerator1"))
      (:B
        (Variables|/Game/MonsterAITest/BP_PatrolPoint.BP_PatrolPoint_C|SetE_PatrolGroup _asbp_patrol_point "NewEnumerator2"))))
  (return PatrolPoints))

(fn GetPatrolPoints
  (params (PatrolGroup :type E_PatrolGroups%20Enum :default "NewEnumerator1") (PatrolPoints :type Array%20of%20BP%20Patrol%20Point%20Object%20References))
  (bind _patrolpointgroup (Variables|Default|GetPatrolPointGroup))
  (for _array_element PatrolPoints
    (bind _asbp_patrol_point (Utilities|Casting|CastToBP_PatrolPoint _array_element))
    (if (Utilities|Enum|Equal(Enum) PatrolGroup (Variables|/Game/MonsterAITest/BP_PatrolPoint.BP_PatrolPoint_C|GetE_PatrolGroup _asbp_patrol_point))
      (Utilities|Array|Add _patrolpointgroup _asbp_patrol_point)))
  (return _patrolpointgroup))