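; Objective log component that keeps track of the active objectives in the quest system.
; AddNewObjective records the quest ID uniquely, then spawns a BP_Objective actor for it and stores the reference, even if the ID is already listed.
; QueryActiveObjective reports whether an ID is active, while CompleteObjective and TrackObjective are empty stubs.
; BeginPlay looks up QuestID in DT_ObjectiveData and prints the objective name.
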(event EventBeginPlay
  (bind _returnvalue (Utilities|GetDataTableRow "/Game/ObjectiveSystem/DT_ObjectiveData.DT_ObjectiveData" (Variables|Default|GetQuestID))
    (:then
      (Development|PrintText (Utilities|Text|ToText(String) (.ObjectiveName (Utilities|Struct|BreakF_ObjectiveDetails _returnvalue))) true true "(R=0.724929,G=0.000000,B=1.000000,A=1.000000)" 1e+01))))

(event EventTick
  (params (DeltaSeconds :type Float%20%28single-precision%29)))

(fn AddNewObjective
  (params (QuestID :type Name%20%28by%20ref%29))
  (Utilities|Array|AddUnique (Variables|Default|GetCurrentActiveObjectives) QuestID)
  (bind _returnvalue (Game|SpawnActorfromClass "/Game/ObjectiveSystem/BP_Objective.BP_Objective_C" (Math|Transform|MakeTransform "0, 0, 0" "0, 0, 0" "1.000000,1.000000,1.000000") "Undefined" "MultiplyWithRoot" 0 QuestID 0))
  (Utilities|Array|Add (Variables|Default|GetCurrentObjectives) _returnvalue))

(fn CompleteObjective)

(fn QueryActiveObjective
  (params (QuestID :type Name))
  (return (Utilities|Array|ContainsItem (Variables|Default|GetCurrentActiveObjectives) QuestID)))

(fn TrackObjective)